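; BP_UDPReceiver is a UDP receive test Blueprint that reacts to incoming data events.
; Each event prints the received Name, Count and Scale on screen in the received Color.
; It also increments its own Count variable and opens the UDPTest1 level once that passes a small fixed threshold.
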(event EventBPEventDataReceived
  (params (ReceivedData :type Custom%20Send%20Data%20Structure%20%28by%20ref%29))
  (bind (_name _count _scale _color) (Utilities|Struct|BreakCustomSendData ReceivedData))
  (Development|PrintString (Utilities|String|ToString(Text) (Utilities|Text|FormatText "Name:{Name}-Count:{Count}-Scale:{Scale}" (Utilities|Text|ToText(String) _name) (Utilities|Text|ToText(Integer) _count) (Utilities|Text|ToText(Float) _scale "HalfToEven"))) true true _color 1.2)
  (Variables|Default|SetCount (+ (Variables|Default|GetCount) 1))
  (if (> (Variables|Default|GetCount) 2)
    (Game|OpenLevel(byName) "UDPTest1")))

(fn ConstructionScript)